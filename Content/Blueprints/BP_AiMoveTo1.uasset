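; BP_AiMoveTo1 is an AI character that continually flees from the first-person player.
; RunAway picks a random reachable point around a spot directly away from the player, moves there with AIMoveTo, and repeats on success or failure.
; When hit by the player, it ragdolls its mesh and destroys its capsule.
; Pressing E separately enables physics simulation on the player's capsule.
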(event `self.ReceiveBeginPlay`
  (bind _asbp_first_person_character (cast `/Game/FirstPerson/Blueprints/BP_FirstPersonCharacter` (`GameplayStatics.GetPlayerCharacter` 0)))
  (set `self.Char REF` _asbp_first_person_character)
  (`self.RunAway`))

(event `RunAway`
  (bind _returnvalue (`self.K2_GetActorLocation`))
  (`|AIMoveTo` self (`NavigationSystemV1.K2_GetRandomReachablePointInRadius` (`KismetMathLibrary.MakeVector` (.x (+ _returnvalue (* (`KismetMathLibrary.GetForwardVector` (`KismetMathLibrary.FindLookAtRotation` _returnvalue (`self.K2_GetActorLocation` (`self.Char REF`)))) -500.0))) (.y (+ _returnvalue (* (`KismetMathLibrary.GetForwardVector` (`KismetMathLibrary.FindLookAtRotation` _returnvalue (`self.K2_GetActorLocation` (`self.Char REF`)))) -500.0))) (.z _returnvalue)) 500.0 null null) null 500.0
    (:`OnSuccess`
      _)
    (:`OnFail`
      _))
  (`self.RunAway`))

(event `self.ReceiveHit`
  (params (MyComp :type "PrimitiveComponent Object Reference") (Other :type "Actor Object Reference") (OtherComp :type "PrimitiveComponent Object Reference") (bSelfMoved :type Boolean) (HitLocation :type "Vector Structure") (HitNormal :type "Vector Structure") (NormalImpulse :type "Vector Structure") (Hit :type "HitResult Structure (by ref)"))
  (cast `/Game/FirstPerson/Blueprints/BP_FirstPersonCharacter` Other)
  (`PrimitiveComponent.SetSimulatePhysics` (`self.Mesh`) true)
  (`ActorComponent.K2_DestroyComponent` (`self.CapsuleComponent`)))

(event `Key|E`
  (params (Key :type "Key Structure"))
  (:`Pressed`
    (`PrimitiveComponent.SetSimulatePhysics` (`Character.CapsuleComponent` (`GameplayStatics.GetPlayerCharacter` 0)) true)))

(fn `UserConstructionScript`)